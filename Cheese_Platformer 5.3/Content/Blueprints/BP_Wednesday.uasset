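; Player-controlled Paper2D character Wednesday for a side-scrolling platformer, with movement along world X, jumping and a score.
; BeginPlay creates the score widget and adds the Enhanced Input mapping; AddPoints updates that widget.
; Jumping plays a fart sound whose volume scales with points; other inputs reload the level, destroy the actor or quit.
; Tick picks flipbooks from ground state and velocity, duplicating the uncalled UpdateAnimation function with an added delay.
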(event Custom|AddPoints
  (params (PointValue :type Integer))
  (Variables|Default|SetPoints (+ PointValue (Variables|Default|GetPoints)))
  (Default|UpdateScore (Variables|Default|GetUI) (Variables|Default|GetPoints)))

(event Input|EnhancedActionEvents|EnhancedInputActionIA_Jump
  (params (ActionValue :type Boolean) (ElapsedSeconds :type Float%20%28double-precision%29) (TriggeredSeconds :type Float%20%28double-precision%29) (InputAction :type Input%20Action%20Object%20Reference :default "/Game/Input/Actions/IA_Jump.IA_Jump"))
  (:Started
    (Character|Jump)
    (Audio|Components|Audio|Play (Variables|Default|GetFart_sound) 0.0))
  (:Completed
    (Character|StopJumping)))

(event Input|EnhancedActionEvents|EnhancedInputActionIA_Move
  (params (ActionValue :type Float%20%28double-precision%29) (ElapsedSeconds :type Float%20%28double-precision%29) (TriggeredSeconds :type Float%20%28double-precision%29) (InputAction :type Input%20Action%20Object%20Reference :default "/Game/Input/Actions/IA_Move.IA_Move"))
  (Pawn|Input|AddMovementInput "1.000000,0.000000,0.000000" ActionValue false)
  (Pawn|SetControlRotation (Pawn|GetController) (select (> ActionValue 0.0) (Math|Rotator|MakeRotator 0.0 0.0 0.0) (Math|Rotator|MakeRotator 0.0 0.0 1.8e+02))))

(event EventBeginPlay
  (Viewport|RemoveAllWidgets)
  (bind _returnvalue (UserInterface|CreateWidget "/Game/Blueprints/UI_Score.UI_Score_C"))
  (bind _output_get (Variables|Default|SetUI _returnvalue))
  (UserInterface|Viewport|AddtoViewport _output_get 0)
  (bind _asplayer_controller (Utilities|Casting|CastToPlayerController (Pawn|GetController)))
  (Input|AddMappingContext (PlayerController|LocalPlayerSubsystems|GetEnhancedInputLocalPlayerSubsystem _asplayer_controller) "/Game/Input/Actions/IMC_Platformer.IMC_Platformer" 0 "(bIgnoreAllPressedKeysUntilRelease=True,bForceImmediately=False,bNotifyUserSettings=False)"))

(event EventTick
  (params (DeltaSeconds :type Float%20%28single-precision%29))
  (Audio|Components|Audio|SetVolumeMultiplier (Variables|Default|GetFart_sound) (* (Math|Conversions|ToFloat(Integer) (Variables|Default|GetPoints)) 0.01) :!class /Script/Engine.AudioComponent)
  (if (AI|Components|NavMovement|IsMovingonGround (Variables|Character|GetCharacterMovement))
    (if (> (Math|Vector|VectorLength (Transformation|GetVelocity)) 0.0)
      (Sprite|SetFlipbook (Variables|Default|GetSprite) "/Game/Assets/Wednesday/Walk_animation/walk_animation.walk_animation")
      (else
        (Sprite|SetFlipbook (Variables|Default|GetSprite) "/Game/Assets/Wednesday/idle_animation/Wednesday_Idle.Wednesday_Idle")))
    (elif (< (.z (Transformation|GetVelocity)) -1e+02)
      (Sprite|SetFlipbook (Variables|Default|GetSprite) "/Game/Assets/Wednesday/Fall_Cont/Fall_Cont.Fall_Cont")
      (else
        (Sprite|SetFlipbook (Variables|Default|GetSprite) "/Game/Assets/Wednesday/Fall_start/Fall_start.Fall_start")
        (Utilities|FlowControl|Delay 1.0)
        (Sprite|SetFlipbook (Variables|Default|GetSprite) "/Game/Assets/Wednesday/Jump_cont_up/Jump_Cont.Jump_Cont")))))

(event Input|ActionEvents|InputActionrestart_game
  (params (Key :type Key%20Structure :default "None"))
  (:Pressed
    (Game|OpenLevel(byName) "Cheese_Platformer_1")))

(event Input|ActionEvents|InputActionrestart_checkpoint
  (params (Key :type Key%20Structure :default "None"))
  (:Pressed
    (Actor|DestroyActor)))

(event Input|ActionEvents|InputActionQuit_button
  (params (Key :type Key%20Structure :default "None"))
  (:Pressed
    (Game|QuitGame 0 "Quit" false)))

(fn ConstructionScript)

(fn UpdateAnimation
  (if (AI|Components|NavMovement|IsMovingonGround (Variables|Character|GetCharacterMovement))
    (if (> (Math|Vector|VectorLength (Transformation|GetVelocity)) 0.0)
      (Sprite|SetFlipbook (Variables|Default|GetSprite) "/Game/Assets/Wednesday/Walk_animation/walk_animation.walk_animation")
      (else
        (Sprite|SetFlipbook (Variables|Default|GetSprite) "/Game/Assets/Wednesday/idle_animation/Wednesday_Idle.Wednesday_Idle")))
    (elif (< (.z (Transformation|GetVelocity)) -1e+02)
      (Sprite|SetFlipbook (Variables|Default|GetSprite) "/Game/Assets/Wednesday/Fall_Cont/Fall_Cont.Fall_Cont")
      (else
        (Sprite|SetFlipbook (Variables|Default|GetSprite) "/Game/Assets/Wednesday/Fall_start/Fall_start.Fall_start")
        (Sprite|SetFlipbook (Variables|Default|GetSprite) "/Game/Assets/Wednesday/Jump_cont_up/Jump_Cont.Jump_Cont")))))