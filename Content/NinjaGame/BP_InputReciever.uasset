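; Input receiver for the Ninja game that damages actors under the mouse cursor while the swipe input is held.
; BeginPlay adds the NinjaInputs mapping context, and AI_Swipe toggles a pressed flag.
; While pressed, each Tick deprojects the viewport-scaled cursor position and runs a short visibility trace from the camera.
; Any hit actor receives a fixed ApplyDamage interface message, repeated every frame it stays under the cursor.
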(event Input|EnhancedActionEvents|EnhancedInputActionAI_Swipe
  (params (ActionValue :type Boolean) (ElapsedSeconds :type Float%20%28double-precision%29) (TriggeredSeconds :type Float%20%28double-precision%29) (InputAction :type Input%20Action%20Object%20Reference :default "/Game/NinjaGame/Inputs/AI_Swipe.AI_Swipe"))
  (:Triggered
    (Variables|Default|SetIsPressingMouse true))
  (:Completed
    (Variables|Default|SetIsPressingMouse false)))

(event EventBeginPlay
  (bind _asplayer_controller (Utilities|Casting|CastToPlayerController (Pawn|GetController)))
  (Input|AddMappingContext (PlayerController|LocalPlayerSubsystems|GetEnhancedInputLocalPlayerSubsystem _asplayer_controller) "/Game/NinjaGame/Inputs/NinjaInputs.NinjaInputs" 0 "(bIgnoreAllPressedKeysUntilRelease=True,bForceImmediately=False,bNotifyUserSettings=False)"))

(event Collision|EventActorBeginOverlap
  (params (OtherActor :type Actor%20Object%20Reference)))

(event EventTick
  (params (DeltaSeconds :type Float%20%28single-precision%29))
  (if (Variables|Default|GetIsPressingMouse)
    (bind (_outhit _returnvalue) (CallFunction|TracetoMouseLocation))
    (if _returnvalue
      (Class|BPIDamagable|ApplyDamage(Message) (.HitActor (Collision|BreakHitResult _outhit)) 5e+01))))

(fn ConstructionScript)

(fn TracetoMouseLocation
  (bind _returnvalue (Game|GetPlayerCameraManager 0))
  (bind _returnvalue_2 (Class|WidgetLayoutLibrary|GetViewportScale))
  (bind _returnvalue_3 (Transformation|GetActorLocation _returnvalue))
  (bind _returnvalue_4 (Class|WidgetLayoutLibrary|GetMousePositiononViewport))
  (bind (_outhit _returnvalue_5) (Collision|LineTraceByChannel _returnvalue_3 (+ _returnvalue_3 (* (.WorldDirection (Class|GameplayStatics|DeprojectScreentoWorld (Game|GetPlayerController 0) (* _returnvalue_4 (Math|Vector|MakeVector _returnvalue_2 _returnvalue_2 0.0)))) 1e+03)) "TraceTypeQuery1" false 0 "None"))
  (return _outhit _returnvalue_5))