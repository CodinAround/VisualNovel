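; Player Blueprint that moves on the world XY plane with WASD, with a visible mouse cursor and a spring-arm zoom.
; Key events set pressed flags, which ProcessMovement reads each Tick to build velocity, divide it by drag and move ParentBox with sweep.
; Tick also adjusts spring-arm length from an input axis value.
; Mouse button flags are recorded but not read in these graphs, and B only logs.
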(event Custom|Process%20Movement
  (bind _velocitydrag (Variables|Default|GetVelocityDrag))
  (bind _movespeed (Variables|Default|GetMoveSpeed))
  ;[0.4922 1 0.3904] Process Movement
  (Utilities|FlowControl|Sequence
    (:then_0
      (Variables|Default|SetXVelocity (+ (+ (* _movespeed (* (Math|Conversions|ToFloat(Boolean) (Variables|Controls|GetPressingLeft)) -1.0)) (* _movespeed (Math|Conversions|ToFloat(Boolean) (Variables|Controls|GetPressingRight)))) (Variables|Default|GetXVelocity)))
      (Variables|Default|SetYVelocity (+ (+ (* _movespeed (* (Math|Conversions|ToFloat(Boolean) (Variables|Controls|GetPressingUp)) -1.0)) (* _movespeed (Math|Conversions|ToFloat(Boolean) (Variables|Controls|GetPressingDown)))) (Variables|Default|GetYVelocity))))
    (:then_1
      (Variables|Default|SetXVelocity (/ (Variables|Default|GetXVelocity) _velocitydrag))
      (Variables|Default|SetYVelocity (/ (Variables|Default|GetYVelocity) _velocitydrag)))
    (:then_2
      (Class|SceneComponent|AddWorldTransform (Variables|Default|GetParentBox) (Math|Transform|MakeTransform (Math|Vector|MakeVector (Variables|Default|GetXVelocity) (Variables|Default|GetYVelocity) 0.0) "0, 0, 0" "1.000000,1.000000,1.000000") true false))))

(event EventBeginPlay
  ;[0.4605 0.2419 1] MAIN INIT
  (Utilities|FlowControl|Sequence
    (:then_0
      (Variables|/Script/Engine.PlayerController|SetbShowMouseCursor (Game|GetPlayerController 0) true))))

(event EventTick
  (params (DeltaSeconds :type Float%20%28single-precision%29))
  ;[1 0.1453 0.1354] MAIN TICK
  (Utilities|FlowControl|Sequence
    (:then_0
      (CallFunction|ProcessMovement))
    (:then_1
      (Variables|/Script/Engine.SpringArmComponent|SetTargetArmLength (Variables|Default|GetSpringArm) (+ (* -2e+01 (Class|Actor|GetInputAxisKeyValue)) (Variables|/Script/Engine.SpringArmComponent|GetTargetArmLength (Variables|Default|GetSpringArm)))))))

(event Input|KeyboardEvents|W
  (params (Key :type Key%20Structure))
  ;[0.8286 0.3558 1] Controls
  (:Pressed
    (Variables|Controls|SetPressingUp true))
  (:Released
    (Variables|Controls|SetPressingUp false)))

(event Input|KeyboardEvents|A
  (params (Key :type Key%20Structure))
  ;[0.8286 0.3558 1] Controls
  (:Pressed
    (Variables|Controls|SetPressingLeft true))
  (:Released
    (Variables|Controls|SetPressingLeft false)))

(event Input|KeyboardEvents|B
  (params (Key :type Key%20Structure))
  ;[0.4605 0.2419 1] MAIN INIT
  (:Pressed
    (Utilities|FlowControl|Sequence
      (:then_0
        (Utilities|String|LogString "pressed b")))))

(event Input|KeyboardEvents|S
  (params (Key :type Key%20Structure))
  ;[0.8286 0.3558 1] Controls
  (:Pressed
    (Variables|Controls|SetPressingDown true))
  (:Released
    (Variables|Controls|SetPressingDown false)))

(event Input|KeyboardEvents|D
  (params (Key :type Key%20Structure))
  ;[0.8286 0.3558 1] Controls
  (:Pressed
    (Variables|Controls|SetPressingRight true))
  (:Released
    (Variables|Controls|SetPressingRight false)))

(event Input|MouseEvents|LeftMouseButton
  (params (Key :type Key%20Structure))
  ;[0.8286 0.3558 1] Controls
  (:Pressed
    (Variables|Controls|SetPressingMouseLeft true))
  (:Released
    (Variables|Controls|SetPressingMouseLeft false)))

(event Input|MouseEvents|MiddleMouseButton
  (params (Key :type Key%20Structure))
  ;[0.8286 0.3558 1] Controls
  (:Pressed
    (Variables|Controls|SetPressingMouseMiddle true))
  (:Released
    (Variables|Controls|SetPressingMouseMiddle false)))

(event Input|MouseEvents|RightMouseButton
  (params (Key :type Key%20Structure))
  ;[0.8286 0.3558 1] Controls
  (:Pressed
    (Variables|Controls|SetPressingMouseRight true))
  (:Released
    (Variables|Controls|SetPressingMouseRight false)))

(event Input|MouseEvents|ThumbMouseButton
  (params (Key :type Key%20Structure))
  ;[0.8286 0.3558 1] Controls
  (:Pressed
    (Variables|Controls|SetPressingMouseThumb1 true))
  (:Released
    (Variables|Controls|SetPressingMouseThumb1 false)))

(event Input|MouseEvents|ThumbMouseButton2
  (params (Key :type Key%20Structure))
  ;[0.8286 0.3558 1] Controls
  (:Pressed
    (Variables|Controls|SetPressingMouseThumb2 true))
  (:Released
    (Variables|Controls|SetPressingMouseThumb2 false)))

(fn ConstructionScript)